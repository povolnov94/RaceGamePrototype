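; Game mode for a checkpoint race against the clock, with a start countdown and a win or lose message.
; On BeginPlay it binds to every BP_Checkpoint, separating the finish line from time-granting checkpoints, and starts the countdown.
; The time limit is a timer handle, re-set with remaining plus bonus time at checkpoints, which also plays a HUD animation.
; Crossing the finish line clears the timer and wins, while expiry loses.
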(event Custom|GameStart
  (bind _returnvalue (Utilities|Time|SetTimerbyEvent (delegate Custom|LoseOutOfTime) (Variables|Default|GetStartTimerDuration)))
  (Variables|Default|SetTimeRemainingTimer _returnvalue))

(event Custom|GameFinish
  (params (IsPlayerWin :type Boolean))
  (Development|PrintString (Utilities|String|SelectString "YouWin" "YouLose" IsPlayerWin) true false "(R=0.000000,G=0.660000,B=1.000000,A=1.000000)" 3.0))

(event Custom|StartCountdown
  (Utilities|FlowControl|Delay (Variables|Default|GetCountdownDuration))
  (CallFunction|GameStart))

(event Custom|LoseOutOfTime
  (CallFunction|GameFinish false))

(event Custom|WinCrossTheFinishLine
  (Utilities|Time|ClearandInvalidateTimerbyHandle (Variables|Default|GetTimeRemainingTimer))
  (CallFunction|GameFinish true))

(event Custom|CrossedCheckpoint
  (params (TimeToAdd :type Integer))
  (CallFunction|AddTimetoTimer TimeToAdd))

(event EventBeginPlay
  (Utilities|FlowControl|Sequence
    (:then_0
      (bind _outactors (Actor|GetAllActorsOfClass "/Game/RaceGame/CheckPoints/BP_Checkpoint.BP_Checkpoint_C"))
      (for _array_element _outactors
        (if (Variables|/Game/RaceGame/CheckPoints/BP_Checkpoint.BP_Checkpoint_C|GetIsFinishLine _array_element)
          (EventDispatchers|BindEventtoOnCheckpointCrossed _array_element (EventDispatchers|CreateEvent :!event Custom|WinCrossTheFinishLine))
          (else
            (EventDispatchers|BindEventtoOnCheckpointCrossedwithTime _array_element (EventDispatchers|CreateEvent :!event Custom|CrossedCheckpoint))))))
    (:then_1
      (CallFunction|StartCountdown))))

(event EventTick
  (params (DeltaSeconds :type Float%20%28single-precision%29)))

(fn ConstructionScript)

(fn AddTimetoTimer
  (params (TimeToAdd :type Integer))
  (bind _returnvalue (Utilities|Time|SetTimerbyEvent (EventDispatchers|CreateEvent :!event Custom|LoseOutOfTime) (+ TimeToAdd (Utilities|Time|GetTimerRemainingTimebyHandle (Variables|Default|GetTimeRemainingTimer)))))
  (Variables|Default|SetTimeRemainingTimer _returnvalue)
  (bind _asvehicle_player_controller (Utilities|Casting|CastToVehiclePlayerController (Game|GetPlayerController 0)))
  (Default|PlayAddedTimeAnim (Variables|/Game/VehicleTemplate/Blueprints/VehiclePlayerController.VehiclePlayerController_C|GetVehicleHud _asvehicle_player_controller)))